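; Base enemy actor that shoots at the player ship and damages it on collision, exploding on impact.
; A construction-sized range sphere enables attacking, and Tick feeds a timed FireProjectiles with rotation that leads the player along X by direction and aim offset.
; When damage drops health below zero, it rolls a weighted random pickup, fires a parting aimed projectile and destroys itself.
; AddMovement offers an unswept location-offset helper.
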(event OnComponentBeginOverlap(firingRangeSphere)
  (params (OverlappedComponent :type Primitive%20Component%20Object%20Reference) (OtherActor :type Actor%20Object%20Reference) (OtherComp :type Primitive%20Component%20Object%20Reference) (OtherBodyIndex :type Integer) (bFromSweep :type Boolean) (SweepResult :type Hit%20Result%20Structure%20%28by%20ref%29))
  (Utilities|Casting|CastTomyPlayerCharacterShip OtherActor)
  (Variables|Default|SetcanAttack true))

(event OnComponentEndOverlap(firingRangeSphere)
  (params (OverlappedComponent :type Primitive%20Component%20Object%20Reference) (OtherActor :type Actor%20Object%20Reference) (OtherComp :type Primitive%20Component%20Object%20Reference) (OtherBodyIndex :type Integer))
  (Utilities|Casting|CastTomyPlayerCharacterShip OtherActor)
  (Variables|Default|SetcanAttack false))

(event Game|Damage|EventAnyDamage
  (params (Damage :type Float%20%28single-precision%29) (DamageType :type Damage%20Type%20Object%20Reference) (InstigatedBy :type Controller%20Object%20Reference) (DamageCauser :type Actor%20Object%20Reference))
  (Variables|Default|Sethealth (- (Variables|Default|Gethealth) Damage))
  (if (< (Variables|Default|Gethealth) 0.0)
    (CallFunction|SpawnRandomItem)
    (Game|SpawnActorfromClass (Variables|Default|Getprojectile) (Math|Transform|MakeTransform (Transformation|GetActorLocation) (Math|Rotator|FindLookatRotation (Transformation|GetActorLocation) (Math|Vector|MakeVector (+ (.x (Transformation|GetActorLocation (stale EventBeginPlay _asmy_player_character_ship))) (* (Variables|/Game/Blueprints/Player/myPlayerCharacterShip.myPlayerCharacterShip_C|Getdirection (stale EventBeginPlay _asmy_player_character_ship)) (Variables|Default|Getaimoffset))) (.y (Transformation|GetActorLocation (stale EventBeginPlay _asmy_player_character_ship))) (.z (Transformation|GetActorLocation (stale EventBeginPlay _asmy_player_character_ship))))) "1,1,1") "Undefined" 0 0)
    (Actor|DestroyActor)))

(event EventBeginPlay
  (bind _asmy_player_character_ship (Utilities|Casting|CastTomyPlayerCharacterShip (Game|GetPlayerCharacter 0))))

(event Collision|EventHit
  (params (MyComp :type Primitive%20Component%20Object%20Reference) (Other :type Actor%20Object%20Reference) (OtherComp :type Primitive%20Component%20Object%20Reference) (bSelfMoved :type Boolean) (HitLocation :type Vector :default "0, 0, 0") (HitNormal :type Vector :default "0, 0, 0") (NormalImpulse :type Vector :default "0, 0, 0") (Hit :type Hit%20Result%20Structure%20%28by%20ref%29))
  (bind _asmy_player_character_ship (Utilities|Casting|CastTomyPlayerCharacterShip Other))
  (Default|DamageSystem _asmy_player_character_ship (Variables|Default|Getdamage))
  (Game|SpawnActorfromClass "/Game/Blueprints/Player/other/explosion.explosion_C" (Transformation|GetActorTransform) "Undefined" 0 0)
  (Actor|DestroyActor))

(event EventTick
  (params (DeltaSeconds :type Float%20%28single-precision%29))
  (CallFunction|FireProjectiles (Math|Rotator|FindLookatRotation (Transformation|GetActorLocation) (Math|Vector|MakeVector (+ (.x (Transformation|GetActorLocation (stale EventBeginPlay _asmy_player_character_ship))) (* (Variables|/Game/Blueprints/Player/myPlayerCharacterShip.myPlayerCharacterShip_C|Getdirection (stale EventBeginPlay _asmy_player_character_ship)) (Variables|Default|Getaimoffset))) (.y (Transformation|GetActorLocation (stale EventBeginPlay _asmy_player_character_ship))) (.z (Transformation|GetActorLocation (stale EventBeginPlay _asmy_player_character_ship))))) DeltaSeconds (Variables|Default|GetfireRate)))

(fn ConstructionScript
  (Components|Sphere|SetSphereRadius (Variables|Default|GetfiringRangeSphere) (Variables|Default|GetfiringRange%20) true))

(fn AddMovement
  (params (movementVector :type Vector))
  (Transformation|SetActorLocation (+ (Transformation|GetActorLocation) movementVector) false false))

(fn FireProjectiles
  (params (SpawnTransform_Rotation :type Rotator) (DeltaSeconds :type Float%20%28single-precision%29) (fireRate :type Float%20%28single-precision%29))
  (if (Variables|Default|GetcanAttack)
    (Variables|Default|Setseconds (+ (Variables|Default|Getseconds) DeltaSeconds))
    (if (> (Variables|Default|Getseconds) fireRate)
      (bind _returnvalue (Game|SpawnActorfromClass (Variables|Default|Getprojectile) (Math|Transform|MakeTransform (Transformation|GetActorLocation) SpawnTransform_Rotation "1,1,1") "Undefined" 0 0))
      (Utilities|Casting|CastToenemyProjectileBase _returnvalue)
      (Variables|Default|Setseconds 0.0))))

(fn SpawnRandomItem
  (bind _returnvalue (Transformation|GetActorTransform))
  (switch int (Math|Random|RandomIntegerinRange 0 15)
    (:4
      (Game|SpawnActorfromClass "/Game/Blueprints/Player/Items/CraftingItems/bp_Orb.bp_Orb_C" _returnvalue "Undefined" 0 0 :!label _label))
    (:5
      (Game|SpawnActorfromClass "/Game/Blueprints/Player/Items/CraftingItems/bp_AiCircuit.bp_AiCircuit_C" _returnvalue "Undefined" 0 0 :!label _label_2))
    (:6
      (Game|SpawnActorfromClass "/Game/Blueprints/Player/Items/CraftingItems/bp_yellowCrystal.bp_yellowCrystal_C" _returnvalue "Undefined" 0 0))
    (:7
      (Game|SpawnActorfromClass "/Game/Blueprints/Player/Items/CraftingItems/bp_blueCrystal.bp_blueCrystal_C" _returnvalue "Undefined" 0 0))
    (:8
      (Game|SpawnActorfromClass "/Game/Blueprints/Player/Items/CraftingItems/bp_Amp.bp_Amp_C" _returnvalue "Undefined" 0 0 :!label _label_3))
    (:9
      (goto _label_2))
    (:10
      (goto _label_3))
    (:11
      (goto _label))))