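; Player ship for a side-scrolling shooter, steered by mouse or touch drag, with quick swipes flipping travel direction.
; Tick eases the ship and a spawned camera along X, then runs turning, fire-rate, speed-heat, shield-recharge and death-state systems.
; Mouse wheel changes speed, which adjusts zoom, touch scale and vertical-scroll lock.
; It also handles two-layer shield damage, inventory pickup, HUD creation, firing toggle and time-slowing menus.
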(event OnComponentBeginOverlap(validateBox)
  (params (OverlappedComponent :type Primitive%20Component%20Object%20Reference) (OtherActor :type Actor%20Object%20Reference) (OtherComp :type Primitive%20Component%20Object%20Reference) (OtherBodyIndex :type Integer) (bFromSweep :type Boolean) (SweepResult :type Hit%20Result%20Structure%20%28by%20ref%29))
  (Utilities|Casting|CastToenemyBase OtherActor))

(event Custom|Dead
  (Game|SpawnActorfromClass "/Game/Blueprints/Player/other/explosion.explosion_C" (Transformation|GetActorTransform) "Undefined" 0 0)
  (Rendering|SetVisibility (Variables|Default|GetStaticMesh) false false)
  (bind _returnvalue (UserInterface|CreateWidget "/Game/Blueprints/Huds/Player/DeadHud.DeadHud_C" (Game|GetPlayerController 0)))
  (Utilities|FlowControl|Delay 0.1)
  (Game|SetGamePaused true)
  (UserInterface|Viewport|AddtoViewport _returnvalue 0))

(event EventBeginPlay
  ;[1 1 1] Camera Work
  (bind _camera (CallFunction|InitializeCamera))
  (Variables|/Script/Engine.PlayerController|SetbShowMouseCursor (Game|GetPlayerController 0) true)
  ;[1 1 1] MainScreen Hud
  (CallFunction|CreateMainHud))

(event EventTick
  (params (DeltaSeconds :type Float%20%28single-precision%29))
  (bind _returnvalue (Transformation|GetActorTransform))
  (bind _returnvalue_2 (Game|GetPlayerController 0))
  (bind _returnvalue_3 (Transformation|GetActorTransform))
  (bind _mainhud (Variables|Default|GetmainHud))
  (bind _camera (Variables|Default|GetCamera))
  (bind _touchstart2d (Variables|Default|GettouchStart2d))
  (bind _returnvalue_4 (Widget|GetOwningPlayer _mainhud))
  (bind (_locationx _locationy) (Game|Player|GetMousePosition _returnvalue_2))
  (bind _returnvalue_5 (Transformation|GetWorldTransform _camera))
  (bind (_location _rotation _scale) (Math|Transform|BreakTransform _returnvalue_3))
  (bind (_sizex _sizey) (HUD|GetViewportSize _returnvalue_4))
  (bind _returnvalue_6 (Math|Vector2D|MakeVector2D _locationx _locationy))
  (bind _returnvalue_7 (- _touchstart2d _returnvalue_6))
  (bind _returnvalue_8 (Math|Vector2D|Vector2DLength _returnvalue_7))
  (Utilities|FlowControl|Sequence
    (:then_0
      (if (Variables|Default|GetbisPressed)
        (Transformation|SetActorTransform (Class|KismetMathLibrary|TInterpto (Math|Transform|MakeTransform (Math|Vector|MakeVector (.x (.location _returnvalue)) 0.0 (.z (.location _returnvalue))) (.rotation _returnvalue) "1,1,1") (Math|Transform|MakeTransform (Math|Vector|MakeVector (+ (.x (.location (Transformation|GetActorTransform (stale EventBeginPlay _camera)))) (* (- _locationx (Math|Conversions|ToFloat(Integer) (/ _sizex 2))) (Variables|Default|GetscreenSizeTouchOffset)) (* 1e+02 (Math|Conversions|ToFloat(Integer) (Variables|Default|Getdirection)))) 0.0 (+ (.z (.location (Transformation|GetActorTransform (stale EventBeginPlay _camera)))) (* (* (- _locationy (Math|Conversions|ToFloat(Integer) (/ _sizey 2))) -1.0) (Variables|Default|GetscreenSizeTouchOffset)) 1e+02)) (.rotation _returnvalue) "1,1,1") DeltaSeconds 5.0))
        (CallFunction|CountSeconds DeltaSeconds (Variables|Default|GettouchSeconds))
        (else
          (Transformation|SetActorTransform (Class|KismetMathLibrary|TInterpto _returnvalue_3 (Math|Transform|MakeTransform (Math|Vector|MakeVector (+ (.x _location) (* (Variables|Default|Getdirection) (/ (Variables|Default|Getspeed) 5.0))) 0.0 (.z _location)) _rotation _scale) DeltaSeconds 5.0)))))
    (:then_1
      ;[1 1 1] Handle Input Controls
      (Utilities|FlowControl|DoOnce false
        (:Completed
          (if (Math|Boolean|ANDBoolean (> _returnvalue_8 75.0) (< _returnvalue_8 7.5e+02) (< (Variables|Default|GettouchSeconds) 0.3))
            (Variables|Default|SettouchSeconds 0.0)
            (Variables|Default|SettouchEnd2d _returnvalue_6)
            (if (not (Variables|Default|GetbRotate))
              (if (> (Math|Float|Absolute(Float) (.X (Math|Vector2D|BreakVector2D (- (Variables|Default|GettouchStart2d) (Variables|Default|GettouchEnd2d))))) (Math|Float|Absolute(Float) (.Y (Math|Vector2D|BreakVector2D (- (Variables|Default|GettouchStart2d) (Variables|Default|GettouchEnd2d))))))
                (if (> (.X (Math|Vector2D|BreakVector2D (- (Variables|Default|GettouchStart2d) (Variables|Default|GettouchEnd2d)))) 0.0)
                  (Development|PrintString "LEFT")
                  (Variables|Default|Setdirection -1)
                  (Variables|Default|SetdodgeRotation "0.000000,0.000000,0.000000" :!label _label)
                  (else
                    (Development|PrintString "RIGHT")
                    (Variables|Default|Setdirection 1)
                    (Variables|Default|SetdodgeRotation "0.000000,0.000000,0.000000" :!label _label_2)))
                (elif (> (.Y (Math|Vector2D|BreakVector2D (- (Variables|Default|GettouchStart2d) (Variables|Default|GettouchEnd2d)))) 0.0)
                  (Development|PrintString "UP")
                  (goto _label_2)
                  (else
                    (Development|PrintString "DOWN")
                    (goto _label))))
              (Variables|Default|SetbRotate true))
            (else
              (Variables|Default|SettouchSeconds 0.0))))))
    (:then_2
      (CallFunction|TurningDIrectionSystem DeltaSeconds)
      (CallFunction|FireRateSystem DeltaSeconds)
      (CallFunction|SpeedOverHeatingSystem DeltaSeconds))
    (:then_3
      ;[1 1 1] Camera Work
      (if (Variables|Default|GetbCanVerticalScroll)
        (Transformation|SetActorTransform (stale EventBeginPlay _camera) (Class|KismetMathLibrary|TInterpto (Transformation|GetActorTransform (stale EventBeginPlay _camera)) (Math|Transform|MakeTransform (Math|Vector|MakeVector (+ (.x (.Location (Math|Transform|BreakTransform (Transformation|GetActorTransform (stale EventBeginPlay _camera))))) (* (Variables|Default|Getdirection) (Variables|Default|Getspeed))) (.y (.location _returnvalue_5)) (.z (.location _returnvalue_5))) (.rotation _returnvalue_5) (.scale _returnvalue_5)) DeltaSeconds 1.0))
        (else
          (Transformation|SetActorTransform (stale EventBeginPlay _camera) (Class|KismetMathLibrary|TInterpto (Transformation|GetActorTransform (stale EventBeginPlay _camera)) (Math|Transform|MakeTransform (Math|Vector|MakeVector (+ (.x (.Location (Math|Transform|BreakTransform (Transformation|GetActorTransform (stale EventBeginPlay _camera))))) (* (Variables|Default|Getdirection) (Variables|Default|Getspeed))) (.y (.location _returnvalue_5)) (Variables|Default|GetNoScrollVerticalHeight)) (.rotation _returnvalue_5) (.scale _returnvalue_5)) DeltaSeconds 1.0))))
      (CallFunction|PlayerStateMachineHandler)
      (Variables|Default|SetCameraLocation (Transformation|GetActorLocation (stale EventBeginPlay _camera)))
      (CallFunction|SheildRechargeSystem DeltaSeconds))))

(event Collision|EventHit
  (params (MyComp :type Primitive%20Component%20Object%20Reference) (Other :type Actor%20Object%20Reference) (OtherComp :type Primitive%20Component%20Object%20Reference) (bSelfMoved :type Boolean) (HitLocation :type Vector :default "0, 0, 0") (HitNormal :type Vector :default "0, 0, 0") (NormalImpulse :type Vector :default "0, 0, 0") (Hit :type Hit%20Result%20Structure%20%28by%20ref%29))
  (Utilities|Casting|CastToprojectileBase Other
    (:CastFailed
      (Camera|PlayWorldCameraShake "/Game/Blueprints/Player/hitCameraShake.hitCameraShake_C" (Transformation|GetActorLocation) 0.0 3e+03))))

(event Input|ActionEvents|InputActionScreenTouch
  (params (Key :type Key%20Structure :default "AnyKey"))
  (bind _returnvalue (Game|GetPlayerController 0))
  (bind (_locationx _locationy) (Game|Player|GetMousePosition _returnvalue))
  (bind _returnvalue_2 (Math|Vector2D|MakeVector2D _locationx _locationy))
  ;[1 1 1] Handle Input Controls
  (:Pressed
    (Variables|Default|SetbisPressed true)
    (Variables|Default|SettouchStart2d _returnvalue_2))
  (:Released
    (Variables|Default|SetbisPressed false)
    (Utilities|FlowControl|DoOnce false) ; enters at Reset
  ))

(event Input|MouseEvents|MiddleMouseButton
  (params (Key :type Key%20Structure :default "AnyKey"))
  (bind _playermessagearmed (Variables|Default|GetPlayerMessageArmed))
  (:Pressed
    (Variables|Default|SetbWeaponWheel true)
    (Variables|Default|SetbFire (not (Variables|Default|GetbFire)))
    (if (not (UserInterface|Viewport|IsinViewport _playermessagearmed))
      (UserInterface|Viewport|AddtoViewport _playermessagearmed 0)))
  (:Released
    (Variables|Default|SetbWeaponWheel false)))

(event Input|MouseEvents|RightMouseButton
  (params (Key :type Key%20Structure :default "AnyKey"))
  (bind _mainhud (Variables|Default|GetmainHud))
  (bind _mainmenuhud (Variables|/Game/Blueprints/Huds/mainHud.mainHud_C|GetmainMenuHud _mainhud))
  (:Pressed
    (if (not (Variables|Default|GetbisPressed))
      (if (UserInterface|Viewport|IsinViewport _mainmenuhud)
        (Default|CloseMenu _mainmenuhud)
        (else
          (UserInterface|Viewport|AddtoViewport _mainmenuhud 0)
          (Utilities|Time|SetGlobalTimeDilation 0.4))))))

(event Input|KeyboardEvents|C
  (params (Key :type Key%20Structure :default "AnyKey"))
  (bind _communicationhud (Variables|Default|GetCommunicationHud))
  (:Pressed
    (if (UserInterface|Viewport|IsinViewport _communicationhud)
      (Widget|RemovefromParent _communicationhud)
      (Utilities|Time|SetGlobalTimeDilation 1.0)
      (else
        (UserInterface|Viewport|AddtoViewport _communicationhud 0)
        (Utilities|Time|SetGlobalTimeDilation 0.005)))))

(event Input|MouseEvents|MouseWheelUp
  (params (Key :type Key%20Structure :default "AnyKey"))
  (bind _springarm (Variables|Default|GetSpringArm))
  (bind _playermessage (Variables|Default|GetplayerMessage))
  (:Pressed
    (if (< (Variables|Default|Getspeed) 1e+02)
      (Variables|Default|Setspeed 3e+02)
      (Variables|/Game/Blueprints/Huds/Player/PlayerMessage.PlayerMessage_C|SetdisplayMessage _playermessage "Speed Up" :!label _label)
      (Variables|/Game/Blueprints/Huds/Player/PlayerMessage.PlayerMessage_C|SetbackgoundColor _playermessage "(R=0.000000,G=1.000000,B=0.034121,A=0.100000)")
      (if (not (UserInterface|Viewport|IsinViewport _playermessage))
        (UserInterface|Viewport|AddtoViewport _playermessage 0)
        (if (< (Variables|Default|Getspeed) 1e+03) :!label _label_2
          (Variables|Default|SetbCanVerticalScroll true)
          (Variables|/Script/Engine.SpringArmComponent|SetTargetArmLength _springarm 2.5e+03)
          (Variables|Default|SetscreenSizeTouchOffset 4.0)
          (else
            (if (Variables|Default|GetbCanVerticalScroll)
              (Variables|Default|SetbCanVerticalScroll false)
              (Variables|Default|SetNoScrollVerticalHeight (.z (Transformation|GetActorLocation))))
            (Variables|/Script/Engine.SpringArmComponent|SetTargetArmLength _springarm 1.4e+03)
            (Variables|Default|SetscreenSizeTouchOffset 2.0))))
      (else
        (Variables|Default|Setspeed (+ (Variables|Default|Getspeed) 3e+02))
        (if (< (Variables|Default|Getspeed) 1.5e+03)
          (goto _label)
          (else
            (Variables|Default|Setspeed 1.5e+03)
            (goto _label_2)))))))

(event Input|MouseEvents|MouseWheelDown
  (params (Key :type Key%20Structure :default "AnyKey"))
  (bind _springarm (Variables|Default|GetSpringArm))
  (bind _playermessage (Variables|Default|GetplayerMessage))
  (:Pressed
    (Variables|Default|Setspeed (- (Variables|Default|Getspeed) 3e+02))
    (if (< (Variables|Default|Getspeed) 1e+02)
      (Variables|Default|Setspeed 1e+01)
      (if (< (Variables|Default|Getspeed) 1e+03) :!label _label
        (Variables|Default|SetbCanVerticalScroll true)
        (Variables|/Script/Engine.SpringArmComponent|SetTargetArmLength _springarm 2.5e+03)
        (Variables|Default|SetscreenSizeTouchOffset 4.0)
        (else
          (if (Variables|Default|GetbCanVerticalScroll)
            (Variables|Default|SetbCanVerticalScroll false)
            (Variables|Default|SetNoScrollVerticalHeight (.z (Transformation|GetActorLocation))))
          (Variables|/Script/Engine.SpringArmComponent|SetTargetArmLength _springarm 1.4e+03)
          (Variables|Default|SetscreenSizeTouchOffset 2.0)))
      (else
        (Variables|/Game/Blueprints/Huds/Player/PlayerMessage.PlayerMessage_C|SetdisplayMessage _playermessage "Speed Down")
        (Variables|/Game/Blueprints/Huds/Player/PlayerMessage.PlayerMessage_C|SetbackgoundColor _playermessage "(R=1.000000,G=0.042226,B=0.000000,A=0.100000)")
        (if (not (UserInterface|Viewport|IsinViewport _playermessage))
          (UserInterface|Viewport|AddtoViewport _playermessage 0)
          (goto _label))))))

(event Input|MouseEvents|LeftMouseButton
  (params (Key :type Key%20Structure :default "AnyKey"))
  (bind _returnvalue (Game|GetPlayerController 0))
  (bind (_locationx _locationy) (Game|Player|GetMousePosition _returnvalue))
  (bind _returnvalue_2 (Math|Vector2D|MakeVector2D _locationx _locationy))
  ;[1 1 1] Handle Input Controls
  (:Pressed
    (Variables|Default|SetbisPressed true)
    (Variables|Default|SettouchStart2d _returnvalue_2))
  (:Released
    (Variables|Default|SetbisPressed false)
    (Utilities|FlowControl|DoOnce false) ; enters at Reset
  ))

(fn ConstructionScript)

(fn InitializeCamera
  (bind _returnvalue (Game|SpawnActorfromClass "/Script/Engine.CameraActor" (Transformation|GetWorldTransform (Variables|Default|GetCamera)) "Undefined" 0 0))
  (Variables|Default|SetmainCamera _returnvalue)
  (Variables|/Script/Engine.CameraComponent|SetbConstrainAspectRatio (Variables|/Script/Engine.CameraActor|GetCameraComponent _returnvalue) true)
  (Game|Player|SetViewTargetwithBlend (Game|GetPlayerController 0) _returnvalue 0.0 "VTBlend_Linear" 0.0 false)
  (return _returnvalue))

(fn SpawnProjectiles
  (params (projectile :type Projectile%20Base%20Class%20Reference) (damage :type Float%20%28single-precision%29))
  (Game|SpawnActorfromClass projectile (Transformation|GetWorldTransform (Variables|Default|GetmainGunBox)) "Undefined" 0 damage 0))

(fn CreateMainHud
  (bind _returnvalue (UserInterface|CreateWidget "/Game/Blueprints/Huds/mainHud.mainHud_C"))
  (Variables|Default|SetmainHud _returnvalue)
  (UserInterface|Viewport|AddtoViewport (Variables|Default|GetmainHud) 0)
  (bind _returnvalue_2 (UserInterface|CreateWidget "/Game/Blueprints/Huds/Player/itemCountHud1.itemCountHud1_C"))
  (Variables|Default|SetitemCountHud1 _returnvalue_2)
  (bind _returnvalue_3 (UserInterface|CreateWidget "/Game/Blueprints/Huds/Player/itemCountHud2.itemCountHud2_C"))
  (Variables|Default|SetitemCountHud2 _returnvalue_3)
  (bind _returnvalue_4 (UserInterface|CreateWidget "/Game/Blueprints/Huds/Player/itemCountHud3.itemCountHud3_C"))
  (Variables|Default|SetitemCountHud3 _returnvalue_4)
  (bind _returnvalue_5 (UserInterface|CreateWidget "/Game/Blueprints/Huds/Player/itemCountHud4.itemCountHud4_C"))
  (Variables|Default|SetitemCountHud4 _returnvalue_5)
  (bind _returnvalue_6 (UserInterface|CreateWidget "/Game/Blueprints/Huds/Player/PlayerMessageArmed.PlayerMessageArmed_C"))
  (Variables|Default|SetPlayerMessageArmed _returnvalue_6)
  (bind _returnvalue_7 (UserInterface|CreateWidget "/Game/Blueprints/Huds/Player/PlayerMessage.PlayerMessage_C"))
  (Variables|Default|SetplayerMessage _returnvalue_7)
  (bind _returnvalue_8 (UserInterface|CreateWidget "/Game/Blueprints/Huds/dialogBoxHud.dialogBoxHud_C"))
  (Variables|Default|SetCommunicationHud _returnvalue_8))

(fn CountSeconds
  (params (DeltaSeconds :type Float%20%28single-precision%29) (count :type Float%20%28single-precision%29%20%28by%20ref%29))
  (|SetBy-RefVar count (+ count DeltaSeconds)))

(fn PrintScreenDebugInfo
  (params (InVec :type Vector%202D%20Structure) (InString :type String))
  (bind _mainhud (Variables|Default|GetmainHud))
  (bind _returnvalue (Widget|GetOwningPlayer _mainhud))
  (bind (_sizex _sizey) (HUD|GetViewportSize _returnvalue))
  (Development|PrintString InString true true "(R=1.000000,G=0.000000,B=0.970272,A=1.000000)")
  (Development|PrintString (Utilities|String|Append "Absolute Screen Cooredinates:    " (Utilities|String|ToString(Vector2d) InVec)))
  (Development|PrintString (Utilities|String|Append "Actor Location:    " (Utilities|String|ToString(Vector) (Transformation|GetActorLocation))) true true "(R=1.000000,G=1.000000,B=0.000000,A=1.000000)")
  (Development|PrintString (Utilities|String|Append "SCREEN SIZE:   " (Utilities|String|BuildString(Integer) "" "X" _sizex "/") (Utilities|String|BuildString(Integer) "" "Y" _sizey)) true true "(R=1.000000,G=0.000000,B=0.038692,A=1.000000)")
  (Development|PrintString "--------" true true "(R=1.000000,G=1.000000,B=1.000000,A=1.000000)"))

(fn PrintSeconds
  (Development|PrintString (Utilities|String|Append "Touch Seconds" (Utilities|String|ToString(Float) (Variables|Default|GettouchSeconds))) true true "(R=0.993651,G=1.000000,B=0.967060,A=1.000000)" 0.0)
  (Development|PrintString (Utilities|String|Append "Rotate Seconds" (Utilities|String|ToString(Float) (Variables|Default|GetrotateSeconds))) true true "(R=0.000000,G=1.000000,B=0.171109,A=1.000000)" 0.0))

(fn AdjustBoxLocations
  (bind _direction (Variables|Default|Getdirection))
  (bind _direction_2 (Variables|Default|Getdirection))
  (bind _maingunbox (Variables|Default|GetmainGunBox))
  (bind _returnvalue (* _direction -1))
  (bind _returnvalue_2 (* _returnvalue 5e+01))
  (Transformation|SetRelativeLocation (Variables|Default|Getoption0Box) (Math|Vector|MakeVector _returnvalue_2 0.0 7e+01) false false)
  (Transformation|SetRelativeLocation (Variables|Default|Getoption1Box) (Math|Vector|MakeVector _returnvalue_2 0.0 -7e+01) false false)
  (Transformation|SetRelativeLocation _maingunbox (Math|Vector|MakeVector (* _direction_2 8e+01) 0.0 0.0) false false)
  (if (> _direction_2 0)
    (Transformation|SetWorldRotation _maingunbox "0, 0, 0" false false)
    (else
      (Transformation|SetWorldRotation _maingunbox "0,180.000000, 0" false false))))

(fn SpeedOverHeatingSystem
  (params (DeltaSeconds :type Float%20%28single-precision%29))
  (bind _speed (Variables|Default|Getspeed))
  (if (Variables|Default|GetbisOnHighway)
    (LocalVariables|SetcooldownValue -0.01 :!label _label)
    (if (> (Variables|Default|GetspeedSeconds) 0.0)
      (CallFunction|CountSeconds (LocalVariables|GetcooldownValue) (Variables|Default|GetspeedSeconds))
      (else
        (Variables|Default|SetspeedSeconds 0.0)
        (Variables|Default|SetbisOverheated false)))
    (elif (> _speed 1.25e+03)
      (if (> _speed 1.5e+03)
        (CallFunction|CountSeconds DeltaSeconds (Variables|Default|GetspeedSeconds))
        (else
          (CallFunction|CountSeconds (/ DeltaSeconds 2.0) (Variables|Default|GetspeedSeconds))))
      (Camera|PlayWorldCameraShake "/Game/Blueprints/Player/speedCameraShake1.speedCameraShake1_C" (Transformation|GetActorLocation) 0.0 3e+03)
      (else
        (goto _label)))))

(fn FireRateSystem
  (params (DeltaSeconds :type Float%20%28single-precision%29))
  (bind _equipedprimaryweapon (Variables|Default|GetequipedPrimaryWeapon))
  (if (and (Variables|Default|GetbFire) (Variables|Default|GetbisPressed))
    (if (> (Variables|Default|GetfireRateSeconds) (.firerate _equipedprimaryweapon))
      (CallFunction|SpawnProjectiles (.projectile _equipedprimaryweapon) (.damage _equipedprimaryweapon))
      (Variables|Default|SetfireRateSeconds 0.0))
    (CallFunction|CountSeconds DeltaSeconds (Variables|Default|GetfireRateSeconds))))

(fn TurningDIrectionSystem
  (params (DeltaTime :type Float%20%28single-precision%29))
  (bind _staticmesh (Variables|Default|GetStaticMesh))
  (bind _returnvalue (Transformation|GetWorldTransform _staticmesh))
  (bind (_location _rotation _scale) (Math|Transform|BreakTransform _returnvalue))
  (CallFunction|AdjustBoxLocations)
  (Transformation|SetWorldTransform _staticmesh (Class|KismetMathLibrary|TInterpto _returnvalue (Math|Transform|MakeTransform _location (Math|Rotator|MakeRotator 0.0 (* (* (Variables|Default|Getdirection) -1) 9e+01) 0.0) _scale) DeltaTime 7.0) false false)
  (if (Variables|Default|GetbRotate)
    (Transformation|AddLocalRotation (Variables|Default|GetStaticMesh) (Variables|Default|GetdodgeRotation) false false)
    (CallFunction|CountSeconds DeltaTime (Variables|Default|GetrotateSeconds))
    (if (> (Variables|Default|GetrotateSeconds) 0.8)
      (Variables|Default|SetbRotate false)
      (Variables|Default|SetrotateSeconds 0.0))))

(fn DamageSystem
  (params (Damage :type Float%20%28single-precision%29))
  (if (> (Variables|Default|GetsecondaryShield) 0.0)
    (Variables|Default|SetsecondaryShield (- (Variables|Default|GetsecondaryShield) (* Damage 3.0)))
    (Variables|Default|SetbisHit true :!label _label)
    (elif (> (Variables|Default|GetmainShield) 0.0)
      (Variables|Default|SetmainShield (- (Variables|Default|GetmainShield) Damage))
      (goto _label)
      (else
        (Variables|Default|SetplayerStates "NewEnumerator1")))))

(fn PlayerStateMachineHandler
  (switch Utilities|FlowControl|Switch|SwitchonplayerStates (Variables|Default|GetplayerStates)
    (:NewEnumerator1
      (CallFunction|Dead))))

(fn SheildRechargeSystem
  (params (DeltaSeconds :type Float%20%28single-precision%29))
  (if (Variables|Default|GetbisHit)
    (Variables|Default|SetbisHit false)
    (Variables|Default|SetsheildSecoends 0.0)
    (elif (< (Variables|Default|GetsheildSecoends) 5.0)
      (CallFunction|CountSeconds DeltaSeconds (Variables|Default|GetsheildSecoends))
      (elif (< (Variables|Default|GetsecondaryShield) 1.0)
        (Variables|Default|SetsecondaryShield (+ (Variables|Default|GetsecondaryShield) DeltaSeconds))))))

(fn AddtoInventory
  (params (item%20master :type Bp%20Item%20Master%20Object%20Reference))
  (bind _itemdata (Variables|/Game/Blueprints/Player/Items/bp_ItemMaster.bp_ItemMaster_C|GetitemData item%20master))
  (bind (_itemname _itemdetails _type _s_weapondetails _s_droiddetails _bcancraft _s_recipedata _bisstackable _weight) (Utilities|Struct|Breaks_ItemData _itemdata))
  (Utilities|Array|Add (Variables|Default|GetitemInventory) (Utilities|Struct|Makes_ItemData _itemname _itemdetails _type _s_weapondetails _s_droiddetails _bcancraft _s_recipedata _bisstackable _weight)))