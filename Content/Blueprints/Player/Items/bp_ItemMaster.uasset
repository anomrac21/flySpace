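; Base pickup item that homes in on the player ship and is collected into its inventory.
; Overlapping FollowTrigger starts a per-tick transform interpolation toward the ship.
; Overlapping CollectTrigger adds the item to inventory, plays a sound, shows a popup and destroys the actor.
; DisplayCollectedWidget cascades through four HUD widgets on the player, using the one matching the item name or the first not in the viewport.
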(event OnComponentBeginOverlap(FollowTrigger)
  (params (OverlappedComponent :type Primitive%20Component%20Object%20Reference) (OtherActor :type Actor%20Object%20Reference) (OtherComp :type Primitive%20Component%20Object%20Reference) (OtherBodyIndex :type Integer) (bFromSweep :type Boolean) (SweepResult :type Hit%20Result%20Structure%20%28by%20ref%29))
  (Utilities|Casting|CastTomyPlayerCharacterShip OtherActor)
  (Variables|Default|SetbCollectItem true))

(event OnComponentBeginOverlap(CollectTrigger)
  (params (OverlappedComponent :type Primitive%20Component%20Object%20Reference) (OtherActor :type Actor%20Object%20Reference) (OtherComp :type Primitive%20Component%20Object%20Reference) (OtherBodyIndex :type Integer) (bFromSweep :type Boolean) (SweepResult :type Hit%20Result%20Structure%20%28by%20ref%29))
  (bind _asmy_player_character_ship (Utilities|Casting|CastTomyPlayerCharacterShip OtherActor))
  (if (== OverlappedComponent (Variables|Default|GetCollectTrigger))
    (Default|AddtoInventory _asmy_player_character_ship self)
    (Audio|PlaySound2D "/Game/Sound/Collectitem.Collectitem")
    (CallFunction|DisplayCollectedWidget)
    (Actor|DestroyActor)))

(event EventTick
  (params (DeltaSeconds :type Float%20%28single-precision%29))
  (if (Variables|Default|GetbCollectItem)
    (bind _asmy_player_character_ship (Utilities|Casting|CastTomyPlayerCharacterShip (Game|GetPlayerCharacter 0)))
    (Transformation|SetActorTransform (Class|KismetMathLibrary|TInterpto (Transformation|GetActorTransform) (Transformation|GetActorTransform _asmy_player_character_ship) DeltaSeconds 6.0))))

(fn ConstructionScript)

(fn DisplayCollectedWidget
  (bind _itemdata (Variables|Default|GetitemData))
  (bind _itemdata_2 (Variables|Default|GetitemData))
  (bind _itemdata_3 (Variables|Default|GetitemData))
  (bind _itemdata_4 (Variables|Default|GetitemData))
  (bind _asmy_player_character_ship (Utilities|Casting|CastTomyPlayerCharacterShip (Game|GetPlayerCharacter 0)))
  ;[1 1 1] Hud 1
  (if (UserInterface|Viewport|IsinViewport (Variables|/Game/Blueprints/Player/myPlayerCharacterShip.myPlayerCharacterShip_C|GetitemCountHud1 _asmy_player_character_ship))
    (if (Utilities|Enum|Equal(Enum) (Variables|/Game/Blueprints/Huds/Player/itemCountHud1.itemCountHud1_C|GetName (Variables|/Game/Blueprints/Player/myPlayerCharacterShip.myPlayerCharacterShip_C|GetitemCountHud1 _asmy_player_character_ship)) (Utilities|Text|ToText(String) (.itemname _itemdata_4)))
      (Variables|/Game/Blueprints/Huds/Player/itemCountHud1.itemCountHud1_C|SetCount (Variables|/Game/Blueprints/Player/myPlayerCharacterShip.myPlayerCharacterShip_C|GetitemCountHud1 _asmy_player_character_ship) "+1")
      (else
        ;[1 1 1] Hud 2
        (if (UserInterface|Viewport|IsinViewport (Variables|/Game/Blueprints/Player/myPlayerCharacterShip.myPlayerCharacterShip_C|GetitemCountHud2 _asmy_player_character_ship))
          (if (Utilities|Enum|Equal(Enum) (Variables|/Game/Blueprints/Huds/Player/itemCountHud2.itemCountHud2_C|GetName (Variables|/Game/Blueprints/Player/myPlayerCharacterShip.myPlayerCharacterShip_C|GetitemCountHud2 _asmy_player_character_ship)) (Utilities|Text|ToText(String) (.itemname _itemdata_3)))
            (Variables|/Game/Blueprints/Huds/Player/itemCountHud2.itemCountHud2_C|SetCount (Variables|/Game/Blueprints/Player/myPlayerCharacterShip.myPlayerCharacterShip_C|GetitemCountHud2 _asmy_player_character_ship) "+1")
            (else
              ;[1 1 1] Hud 3
              (if (UserInterface|Viewport|IsinViewport (Variables|/Game/Blueprints/Player/myPlayerCharacterShip.myPlayerCharacterShip_C|GetitemCountHud3 _asmy_player_character_ship))
                (if (Utilities|Enum|Equal(Enum) (Variables|/Game/Blueprints/Huds/Player/itemCountHud3.itemCountHud3_C|GetName (Variables|/Game/Blueprints/Player/myPlayerCharacterShip.myPlayerCharacterShip_C|GetitemCountHud3 _asmy_player_character_ship)) (Utilities|Text|ToText(String) (.itemname _itemdata_2)))
                  (Variables|/Game/Blueprints/Huds/Player/itemCountHud3.itemCountHud3_C|SetCount (Variables|/Game/Blueprints/Player/myPlayerCharacterShip.myPlayerCharacterShip_C|GetitemCountHud3 _asmy_player_character_ship) "+1")
                  (else
                    ;[1 1 1] Hud 4
                    (if (UserInterface|Viewport|IsinViewport (Variables|/Game/Blueprints/Player/myPlayerCharacterShip.myPlayerCharacterShip_C|GetitemCountHud4 _asmy_player_character_ship))
                      (if (Utilities|Enum|Equal(Enum) (Variables|/Game/Blueprints/Huds/Player/itemCountHud4.itemCountHud4_C|GetName (Variables|/Game/Blueprints/Player/myPlayerCharacterShip.myPlayerCharacterShip_C|GetitemCountHud4 _asmy_player_character_ship)) (Utilities|Text|ToText(String) (.itemname _itemdata)))
                        (Variables|/Game/Blueprints/Huds/Player/itemCountHud4.itemCountHud4_C|SetCount (Variables|/Game/Blueprints/Player/myPlayerCharacterShip.myPlayerCharacterShip_C|GetitemCountHud4 _asmy_player_character_ship) "+1"))
                      (else
                        (Variables|/Game/Blueprints/Huds/Player/itemCountHud4.itemCountHud4_C|SetName (Variables|/Game/Blueprints/Player/myPlayerCharacterShip.myPlayerCharacterShip_C|GetitemCountHud4 _asmy_player_character_ship) (Utilities|Text|ToText(String) (.itemname _itemdata)))
                        (Variables|/Game/Blueprints/Huds/Player/itemCountHud4.itemCountHud4_C|SetCount (Variables|/Game/Blueprints/Player/myPlayerCharacterShip.myPlayerCharacterShip_C|GetitemCountHud4 _asmy_player_character_ship) "+1")
                        (Variables|/Game/Blueprints/Huds/Player/itemCountHud4.itemCountHud4_C|SetColor (Variables|/Game/Blueprints/Player/myPlayerCharacterShip.myPlayerCharacterShip_C|GetitemCountHud4 _asmy_player_character_ship) (Variables|Default|GetwidgetColor))
                        (UserInterface|Viewport|AddtoViewport (Variables|/Game/Blueprints/Player/myPlayerCharacterShip.myPlayerCharacterShip_C|GetitemCountHud4 _asmy_player_character_ship) 0)))))
                (else
                  (Variables|/Game/Blueprints/Huds/Player/itemCountHud3.itemCountHud3_C|SetName (Variables|/Game/Blueprints/Player/myPlayerCharacterShip.myPlayerCharacterShip_C|GetitemCountHud3 _asmy_player_character_ship) (Utilities|Text|ToText(String) (.itemname _itemdata_2)))
                  (Variables|/Game/Blueprints/Huds/Player/itemCountHud3.itemCountHud3_C|SetCount (Variables|/Game/Blueprints/Player/myPlayerCharacterShip.myPlayerCharacterShip_C|GetitemCountHud3 _asmy_player_character_ship) "+1")
                  (Variables|/Game/Blueprints/Huds/Player/itemCountHud3.itemCountHud3_C|SetColor (Variables|/Game/Blueprints/Player/myPlayerCharacterShip.myPlayerCharacterShip_C|GetitemCountHud3 _asmy_player_character_ship) (Variables|Default|GetwidgetColor))
                  (UserInterface|Viewport|AddtoViewport (Variables|/Game/Blueprints/Player/myPlayerCharacterShip.myPlayerCharacterShip_C|GetitemCountHud3 _asmy_player_character_ship) 0)))))
          (else
            (Variables|/Game/Blueprints/Huds/Player/itemCountHud2.itemCountHud2_C|SetName (Variables|/Game/Blueprints/Player/myPlayerCharacterShip.myPlayerCharacterShip_C|GetitemCountHud2 _asmy_player_character_ship) (Utilities|Text|ToText(String) (.itemname _itemdata_3)))
            (Variables|/Game/Blueprints/Huds/Player/itemCountHud2.itemCountHud2_C|SetCount (Variables|/Game/Blueprints/Player/myPlayerCharacterShip.myPlayerCharacterShip_C|GetitemCountHud2 _asmy_player_character_ship) "+1")
            (Variables|/Game/Blueprints/Huds/Player/itemCountHud2.itemCountHud2_C|SetColor (Variables|/Game/Blueprints/Player/myPlayerCharacterShip.myPlayerCharacterShip_C|GetitemCountHud2 _asmy_player_character_ship) (Variables|Default|GetwidgetColor))
            (UserInterface|Viewport|AddtoViewport (Variables|/Game/Blueprints/Player/myPlayerCharacterShip.myPlayerCharacterShip_C|GetitemCountHud2 _asmy_player_character_ship) 0)))))
    (else
      (Variables|/Game/Blueprints/Huds/Player/itemCountHud1.itemCountHud1_C|SetName (Variables|/Game/Blueprints/Player/myPlayerCharacterShip.myPlayerCharacterShip_C|GetitemCountHud1 _asmy_player_character_ship) (Utilities|Text|ToText(String) (.itemname _itemdata_4)))
      (Variables|/Game/Blueprints/Huds/Player/itemCountHud1.itemCountHud1_C|SetCount (Variables|/Game/Blueprints/Player/myPlayerCharacterShip.myPlayerCharacterShip_C|GetitemCountHud1 _asmy_player_character_ship) "+1")
      (Variables|/Game/Blueprints/Huds/Player/itemCountHud1.itemCountHud1_C|SetColor (Variables|/Game/Blueprints/Player/myPlayerCharacterShip.myPlayerCharacterShip_C|GetitemCountHud1 _asmy_player_character_ship) (Variables|Default|GetwidgetColor))
      (UserInterface|Viewport|AddtoViewport (Variables|/Game/Blueprints/Player/myPlayerCharacterShip.myPlayerCharacterShip_C|GetitemCountHud1 _asmy_player_character_ship) 0)))
  (Audio|PlaySound2D "/Game/Sound/Collectitem.Collectitem")
  (Actor|DestroyActor))