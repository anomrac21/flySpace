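; Background stars Blueprint that tiles a static mesh into a flat grid.
; The construction script runs nested loops over Width and Height, adding one InstancedStaticMesh instance per cell with a fixed rotation and unit scale.
; Despite their names, YOffset spaces the instances along X and ZOffset along Y, with Z held at zero.
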(fn ConstructionScript
  (for _index (range 0 (Variables|Default|Getwidth))
    (for _index_2 (range 0 (Variables|Default|Getheight))
      (Components|InstancedStaticMesh|AddInstance (Variables|Default|GetInstancedStaticMesh) (Math|Transform|MakeTransform (Math|Vector|MakeVector (Math|Conversions|ToFloat(Integer) (* _index (Variables|Default|GetyOffset))) (Math|Conversions|ToFloat(Integer) (* _index_2 (Variables|Default|GetzOffset))) 0.0) "90.000000, 0,0.000000")))))