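; SpeedHighway is an environment actor that marks the player ship as on the highway and suppresses firing there.
; The construction script builds it from a row of rotated mesh instances along X, set by Width and XOffset.
; Overlapping RightDirectionBox toggles BisOnHighway on the ship.
; While that flag is set, Tick clears any Fire input and shows the ship's PlayerMessageArmed widget.
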(event OnComponentEndOverlap(RightDirectionBox)
  (params (OverlappedComponent :type Primitive%20Component%20Object%20Reference) (OtherActor :type Actor%20Object%20Reference) (OtherComp :type Primitive%20Component%20Object%20Reference) (OtherBodyIndex :type Integer))
  (bind _asmy_player_character_ship (Utilities|Casting|CastTomyPlayerCharacterShip OtherActor))
  (Variables|/Game/Blueprints/Player/myPlayerCharacterShip.myPlayerCharacterShip_C|SetbisOnHighway _asmy_player_character_ship false))

(event OnComponentBeginOverlap(RightDirectionBox)
  (params (OverlappedComponent :type Primitive%20Component%20Object%20Reference) (OtherActor :type Actor%20Object%20Reference) (OtherComp :type Primitive%20Component%20Object%20Reference) (OtherBodyIndex :type Integer) (bFromSweep :type Boolean) (SweepResult :type Hit%20Result%20Structure%20%28by%20ref%29))
  (bind _asmy_player_character_ship (Utilities|Casting|CastTomyPlayerCharacterShip OtherActor))
  (Variables|/Game/Blueprints/Player/myPlayerCharacterShip.myPlayerCharacterShip_C|SetbisOnHighway _asmy_player_character_ship true))

(event EventTick
  (params (DeltaSeconds :type Float%20%28single-precision%29))
  (bind _character (Variables|Default|GetCharacter))
  (bind _playermessagearmed (Variables|/Game/Blueprints/Player/myPlayerCharacterShip.myPlayerCharacterShip_C|GetPlayerMessageArmed _character))
  (if (Variables|/Game/Blueprints/Player/myPlayerCharacterShip.myPlayerCharacterShip_C|GetbisOnHighway _character)
    (if (Variables|/Game/Blueprints/Player/myPlayerCharacterShip.myPlayerCharacterShip_C|GetbFire _character)
      (Variables|/Game/Blueprints/Player/myPlayerCharacterShip.myPlayerCharacterShip_C|SetbFire _character false)
      (if (not (UserInterface|Viewport|IsinViewport _playermessagearmed))
        (UserInterface|Viewport|AddtoViewport _playermessagearmed 0)))))

(event EventBeginPlay
  (bind _asmy_player_character_ship (Utilities|Casting|CastTomyPlayerCharacterShip (Game|GetPlayerCharacter 0)))
  (Variables|Default|SetCharacter _asmy_player_character_ship))

(fn ConstructionScript
  (bind _instancedstaticmesh (Variables|Default|GetInstancedStaticMesh))
  (for _index (range 0 (Variables|Default|Getwidth))
    (bind _returnvalue (Components|InstancedStaticMesh|AddInstance _instancedstaticmesh (Math|Transform|MakeTransform (Math|Vector|MakeVector (Math|Conversions|ToFloat(Integer) (* _index (Variables|Default|GetxOffset))) 0.0 0.0) "90.000000, 0,0.000000")))
    (Rendering|Material|SetMaterial _instancedstaticmesh _returnvalue (Variables|Default|GetMaterial))))